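; BP_Tile is a terrain segment for infinite terrain, with a barrier gate that reacts to the player character.
; The barrier starts locked (solid, red), opens (no collision, green) inside the locking volume, and relocks on exit.
; Leaving that volume also asks GM_InfiniteTerrain to spawn a tile, while entering the destroy volume removes this one.
; An Arrow component exposes the attach transform for tiles.
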(event `self.ReceiveBeginPlay`
  (`self.Lock`))

(event `self.LockingVolume.OnComponentBeginOverlap`
  (params (OverlappedComponent :type "PrimitiveComponent Object Reference") (OtherActor :type "Actor Object Reference") (OtherComp :type "PrimitiveComponent Object Reference") (OtherBodyIndex :type Integer) (bFromSweep :type Boolean) (SweepResult :type "HitResult Structure (by ref)"))
  (`self.IsPlayerActor` OtherActor)
  (`self.Unlock`))

(event `self.LockingVolume.OnComponentEndOverlap`
  (params (OverlappedComponent :type "PrimitiveComponent Object Reference") (OtherActor :type "Actor Object Reference") (OtherComp :type "PrimitiveComponent Object Reference") (OtherBodyIndex :type Integer))
  (`self.IsPlayerActor` OtherActor)
  (`self.Lock`)
  (`/Game/Dynamic/GM_InfiniteTerrain.SpawnTile` (cast `/Game/Dynamic/GM_InfiniteTerrain` (`GameplayStatics.GetGameMode`) :!pure true)))

(event `self.DestroyVolume.OnComponentBeginOverlap`
  (params (OverlappedComponent :type "PrimitiveComponent Object Reference") (OtherActor :type "Actor Object Reference") (OtherComp :type "PrimitiveComponent Object Reference") (OtherBodyIndex :type Integer) (bFromSweep :type Boolean) (SweepResult :type "HitResult Structure (by ref)"))
  (`self.IsPlayerActor` OtherActor)
  (`self.K2_DestroyActor`))

(fn `Get AttachTransform`
  (returns (AttachTransform :type "Transform Structure"))
  (return (`SceneComponent.K2_GetComponentToWorld` (`self.Arrow`))))

(fn `Lock`
  (bind _barrier (`self.Barrier`))
  (`PrimitiveComponent.SetCollisionEnabled` _barrier "QueryAndPhysics")
  (`PrimitiveComponent.SetMaterial` _barrier 0 "/Game/Dynamic/Terrain/MI_BarrierRed.MI_BarrierRed"))

(fn `Unlock`
  (bind _barrier (`self.Barrier`))
  (`PrimitiveComponent.SetCollisionEnabled` _barrier "NoCollision")
  (`PrimitiveComponent.SetMaterial` _barrier 0 "/Game/Dynamic/Terrain/MI_BarrierGreen.MI_BarrierGreen"))

(fn `UserConstructionScript`)